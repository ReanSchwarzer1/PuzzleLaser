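; BP_StairDoor is an activatable puzzle actor that raises and lowers a set of stairs through Up and Down interface events.
; A timeline drives the Z world scale of the Stairs component, playing forward for up and reversing for down.
; On BeginPlay it plays the up animation if the Up flag is set.
; Its IsActorActivated interface function always returns false.
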(event `self.Up_BPI`
  ;[1 1 1] Trigger action up/ down
  (bind (_direction _track) (`Timeline|Timeline_Open` :!label _label)
    (:`Update`
      (`SceneComponent.SetWorldScale3D` (`self.Stairs`) (`KismetMathLibrary.MakeVector` (`self.New Scale X`) (`self.New Scale Y`) _track)))))

(event `self.Down_BPI`
  ;[1 1 1] Trigger action up/ down
  (goto _label :!via `Reverse`))

(event `self.ReceiveBeginPlay`
  ;[1 1 1] Set Stairs in up position
  (if (`self.Up?`)
    (`self.Up_BPI`)))

(fn `IsActorActivated_BPI`
  (returns (Activated :type Boolean))
  (return false))

(fn `UserConstructionScript`)